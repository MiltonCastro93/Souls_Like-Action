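; Actor component that holds a character's combat state: main weapon, combat mode and attack progress.
; Setting a main weapon first unequips and destroys any valid current one, so only one exists at a time.
; Toggling combat mode immediately notifies the owning character's AnimInstance through an interface message.
; A reset function clears the attack count, saved-attack flag and attacking flag.
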(event EventBeginPlay)

(event EventTick
  (params (DeltaSeconds :type Float%20%28single-precision%29)))

(fn SetMainWeapon
  (params (NewWeapon :type BP%20Base%20Weapon%20Object%20Reference))
  ;[0 0 0 0.5] De esta manera me sera imposible tener mas de un arma
  (Utilities|FlowControl|Sequence
    (:then_0
      (Utilities|IsValid (Variables|Default|GetMainWeapon)
        (:Is%20Valid
          (Default|OnUnEquipped (Variables|Default|GetMainWeapon))
          (Actor|DestroyActor (Variables|Default|GetMainWeapon)))))
    (:then_1
      (Variables|Default|SetMainWeapon NewWeapon))))

(fn GetMainWeapon
  (return (Variables|Default|GetMainWeapon)))

(fn SetCombatEnable
  (params (CombatEnable :type Boolean))
  (bind _output_get (Variables|Default|SetCombat%20Enable? CombatEnable))
  ;[0 0 0 0.5] Obtengo la Interface para actualizar al instante
  (Class|BPIAnimInstance|UpdateCombatEnable(Message) (Components|SkeletalMesh|GetAnimInstance (Variables|/Script/Engine.Character|GetMesh (.AsCharacter (Utilities|Casting|CastToCharacter (Components|GetOwner))))) _output_get))

(fn IsCombatEnable?
  (return (Variables|Default|GetCombat%20Enable?)))

(fn ResetAttack
  (Variables|Default|SetAttackCount 0)
  (Variables|Default|SetIsAttachSaved? false)
  (Variables|Default|SetIsAttacking false))