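; BP_BaseWeapon is the base weapon Blueprint in the combat system, extending BP_BaseEquippable.
; On equip, it registers itself as the owning BP_Combatiente's MainWeapon and sends its CombatType to that character's AnimInstance.
; SetAttachedToHand stores the in-hand state and forwards it to the AnimInstance through an interface message, while IsAttackedToHand? returns that state.
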(event EventBeginPlay
  (|CallParentFunction) ; This node is disabled and will not be called.\nDrag off pins to build functionality.
)

(event Collision|EventActorBeginOverlap
  (params (OtherActor :type Actor%20Object%20Reference))
  (|CallParentFunction OtherActor) ; This node is disabled and will not be called.\nDrag off pins to build functionality.
)

(event EventTick
  (params (DeltaSeconds :type Float%20%28single-precision%29))
  (|CallParentFunction DeltaSeconds) ; This node is disabled and will not be called.\nDrag off pins to build functionality.
)

(fn ConstructionScript
  (|CallParentFunction))

(fn OnEquipped
  ;[0 0 0 0.5] Le agrego mas funcionalidad Haciendole Overrider a la Clase Padre "BP_BaseEquippable"
  (|CallParentFunction)
  (bind _asbp_combatiente (Utilities|Casting|CastToBP_Combatiente (Components|GetOwner)))
  (Variables|/Game/CombateSystem/Blueprints/BP_Combatiente.BP_Combatiente_C|SetMainWeapon _asbp_combatiente self)
  (Class|BPIAnimInstance|UpdateCombatType(Message) (Components|SkeletalMesh|GetAnimInstance (Variables|/Script/Engine.Character|GetMesh _asbp_combatiente)) (Variables|Initialization|GetCombatType)))

(fn SetAttachedtoHand
  (params (inModeAttach? :type Boolean))
  (Variables|Default|SetinModeAttach? inModeAttach?)
  (bind _asbp_combatiente (Utilities|Casting|CastToBP_Combatiente (Components|GetOwner)))
  ;[0.15 0.15 0.15 0.5] Interfaces proveniente del ABP_Unarmed
  (Class|BPIAnimInstance|UpdateWeaponAttachedtoHand(Message) (Components|SkeletalMesh|GetAnimInstance (Variables|/Script/Engine.Character|GetMesh _asbp_combatiente)) (Variables|Default|GetinModeAttach?)))

(fn IsAttackedtoHand?
  (return (Variables|Default|GetinModeAttach?)))